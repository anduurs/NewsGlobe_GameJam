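; PlayerPawn is a player pawn that detects which InteractAble actor sits under the mouse cursor and drives its hover state.
; Each Tick it line-traces on the Visibility channel from the deprojected cursor position to an end point scaled from the cursor direction, without adding the start position.
; When the hit actor changes, it calls HoverEnd and HoverBegin as needed and caches or clears the current Interactable.
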(event `self.ReceiveTick`
  (params (DeltaSeconds :type "Float (single-precision)"))
  (bind _returnvalue (`GameplayStatics.GetPlayerController` 0))
  (bind _interactable (`self.interactable`))
  (bind _interactable_2 (`self.interactable`))
  (bind (_worldlocation _worlddirection) (`PlayerController.DeprojectMousePositionToWorld` _returnvalue))
  (bind _outhit (`KismetSystemLibrary.LineTraceSingle` _worldlocation (* _worlddirection (+ (`KismetMathLibrary.GetForwardVector` (`Controller.GetControlRotation` _returnvalue)) 12000.0)) "TraceTypeQuery1"))
  (bind (_bblockinghit _binitialoverlap _time _location _impactpoint _normal _impactnormal _physmat _hitactor) (`GameplayStatics.BreakHitResult` _outhit))
  (if (not (== (`self.interactable`) _hitactor))
    (bind _asinteract_able (cast `/Game/Blueprints/InteractAble` _hitactor)
      (:`then`
        (`/Engine/EditorBlueprintResources/StandardMacros.IsValid` _interactable
          (:`Is Valid`
            (`/Game/Blueprints/InteractAble.Hover End` _interactable))
          (:`Is Not Valid`
            _))
        (`/Game/Blueprints/InteractAble.Hover Begin` _asinteract_able)
        (set `self.interactable` _asinteract_able))
      (:`CastFailed`
        (`/Engine/EditorBlueprintResources/StandardMacros.IsValid` _interactable_2
          (:`Is Valid`
            (`/Game/Blueprints/InteractAble.Hover End` _interactable_2)
            (set `self.interactable` null)))))))

(fn `UserConstructionScript`)