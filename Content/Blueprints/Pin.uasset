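; Pin is an interactive actor that highlights on hover and toggles a clicked state when the player interacts with it.
; BeginPlay creates dynamic materials for both mesh slots and binds OnInteract to the GameController's interact dispatcher.
; Hover events show or hide PinHoverActor and switch the materials' Flashing parameter.
; An interact press only calls Click while hovered, where a FlipFlop alternates the Clicked variable.
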(event `self.ReceiveBeginPlay`
  (bind _staticmesh (`self.StaticMesh`))
  (bind _returnvalue (`PrimitiveComponent.CreateDynamicMaterialInstance` _staticmesh 0 (`PrimitiveComponent.GetMaterial` _staticmesh 0)))
  (set `self.DynamicPinMat1` _returnvalue)
  (bind _returnvalue_2 (`PrimitiveComponent.CreateDynamicMaterialInstance` _staticmesh 1 (`PrimitiveComponent.GetMaterial` _staticmesh 1)))
  (set `self.DynamicPinMat2` _returnvalue_2)
  (bind _asgame_controller (cast `/Game/Blueprints/GameController` (`GameplayStatics.GetPlayerController` 0)))
  (add `/Game/Blueprints/GameController.InteractDispatcher` _asgame_controller (delegate `OnInteract`)))

(event `OnInteract`
  (params (Clicked :type Boolean))
  (if (and Clicked (`self.Hoover`))
    (`self.Click`)))

(event `self.Click`
  (`/Engine/EditorBlueprintResources/StandardMacros.FlipFlop`
    (:`A`
      (set `self.Clicked` true))
    (:`B`
      (set `self.Clicked` false))))

(event `self.Hover Begin`
  (`SceneComponent.SetVisibility` (`self.PinHoverActor`) true true)
  (set `self.Hoover` true)
  (`MaterialInstanceDynamic.SetScalarParameterValue` (`self.DynamicPinMat1`) "Flashing" 1.0)
  (`MaterialInstanceDynamic.SetScalarParameterValue` (`self.DynamicPinMat2`) "Flashing" 1.0))

(event `self.Hover End`
  (`SceneComponent.SetVisibility` (`self.PinHoverActor`) false true)
  (set `self.Hoover` false)
  (`MaterialInstanceDynamic.SetScalarParameterValue` (`self.DynamicPinMat1`) "Flashing" 0.0)
  (`MaterialInstanceDynamic.SetScalarParameterValue` (`self.DynamicPinMat2`) "Flashing" 0.0))

(fn `UserConstructionScript`)