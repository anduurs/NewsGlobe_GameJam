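; Player controller that drives an orbit-style camera, apparently around an Earth globe, by rotating and zooming the PlayerPawn.
; While the left mouse button is held, axis input rotates the pawn with clamped pitch and is stored as spin speed, which coasts with linear decay after release.
; The mouse wheel adjusts clamped spring arm length and derives ScaleFactor from it.
; Press and release also fire an interact dispatcher.
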(event `self.ReceiveBeginPlay`
  (bind _asplayer_pawn (cast `/Game/Blueprints/PlayerPawn` (`GameplayStatics.GetPlayerPawn` 0)))
  (set `self.Player Pawn` _asplayer_pawn))

(event `self.ReceiveTick`
  (params (DeltaSeconds :type "Float (single-precision)"))
  (bind _returnvalue (`GameplayStatics.GetPlayerPawn` 0))
  (bind _returnvalue_2 (`self.GetInputAxisKeyValue`))
  (bind _returnvalue_3 (`self.GetInputAxisKeyValue`))
  (bind (_earthspinspeed_roll _earthspinspeed_pitch _earthspinspeed_yaw) (`KismetMathLibrary.BreakRotator` (`self.EarthSpinSpeed`)))
  (bind _earthspinspeed (`self.EarthSpinSpeed`))
  (bind (_returnvalue_roll _returnvalue_pitch _returnvalue_yaw) (`KismetMathLibrary.BreakRotator` (`self.K2_GetActorRotation` _returnvalue)))
  (bind _returnvalue_4 (`KismetMathLibrary.VSize` _earthspinspeed))
  (if (`self.Left Mouse Button Down`)
    (`self.K2_SetActorRotation` _returnvalue (`KismetMathLibrary.MakeRotator` 0.0 (`KismetMathLibrary.FClamp` (+ _returnvalue_pitch _returnvalue_3) -70.0 70.0) (+ _returnvalue_yaw _returnvalue_2)) false)
    (set `self.EarthSpinSpeed` (`KismetMathLibrary.MakeRotator` 0.0 _returnvalue_3 _returnvalue_2))
    (else
      (`self.K2_SetActorRotation` (`self.Player Pawn`) (`KismetMathLibrary.MakeRotator` 0.0 (`KismetMathLibrary.FClamp` (+ _returnvalue_pitch _earthspinspeed_pitch) -70.0 70.0) (+ _returnvalue_yaw _earthspinspeed_yaw)) false)
      (`/Engine/EditorBlueprintResources/StandardMacros.CompareFloat` _returnvalue_4 0.1
        (:`>`
          (set `self.EarthSpinSpeed` (* (`KismetMathLibrary.Normal` _earthspinspeed) (- _returnvalue_4 0.1))))
        (:`==`
          (set `self.EarthSpinSpeed` (0.0 0.0 0.0) :!label _label))
        (:`<`
          (goto _label))))))

(event `InputAxisKey|MouseWheelAxis`
  (params (AxisValue :type "Float (single-precision)"))
  (bind _springarm (`/Game/Blueprints/PlayerPawn.SpringArm` (`self.Player Pawn`)))
  (bind _output_get (set `SpringArmComponent.TargetArmLength` (`KismetMathLibrary.FClamp` (+ (* AxisValue -50.0) (`SpringArmComponent.TargetArmLength` _springarm)) 600.0 1500.0) _springarm))
  (set `self.ScaleFactor` (/ _output_get 1000.0)))

(event `Key|LeftMouseButton`
  (params (Key :type "Key Structure"))
  (:`Pressed`
    (`self.InteractDispatcher` true)
    (set `self.Left Mouse Button Down` true))
  (:`Released`
    (`self.InteractDispatcher` false)
    (set `self.Left Mouse Button Down` false)))

(fn `UserConstructionScript`)