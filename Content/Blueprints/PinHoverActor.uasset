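; Hover panel actor that shows a location name and its news headlines as link actors.
; InitObject sets the name text and spawns one LinkActor per headline, paired with its URL, attached to BG in an evenly spaced stack.
; BeginPlay fills it with test data, and Tick turns the actor to face the player pawn's camera.
; An older fixed five-slot text update remains as unconnected nodes.
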(event `self.ReceiveBeginPlay`
  (`self.InitObject` (`self.TestTitles`) "SKÖVDE" (`self.TestLinks`)))

(event `self.ReceiveTick`
  (params (DeltaSeconds :type "Float (single-precision)"))
  (bind _asplayer_pawn (cast `/Game/Blueprints/PlayerPawn` (`GameplayStatics.GetPlayerPawn` 0)))
  (`self.K2_SetActorRotation` (`KismetMathLibrary.FindLookAtRotation` (`self.K2_GetActorLocation`) (`SceneComponent.K2_GetComponentLocation` (`/Game/Blueprints/PlayerPawn.Camera` _asplayer_pawn)))))

(fn `InitObject`
  (params (NewsHeaders :type "Array of String") (LocationName :type String) (Links :type "Array of String"))
  (`self.UpdateLocationName` LocationName)
  (`self.UpdateNewsHeaders` NewsHeaders Links))

(fn `UpdateLocationName`
  (params (LocationName :type String))
  (`TextRenderComponent.K2_SetText` (`self.LocationName`) (`KismetTextLibrary.Conv_StringToText` LocationName)))

(fn `UpdateNewsHeaders`
  (params (NewsHeaders :type "Array of String") (Links :type "Array of String"))
  (for (_array_element _array_index) NewsHeaders
    (bind _returnvalue (`|SpawnActorFromClass` "/Game/Blueprints/LinkActor.LinkActor_C" (`KismetMathLibrary.MakeTransform` (0.0 0.0 0.0)) "AlwaysSpawn" "OverrideRootScale" null _array_element (`|GetArrayItem` Links _array_index) null))
    (`self.K2_AttachToComponent` _returnvalue (`self.BG`) "None" "SnapToTarget" "SnapToTarget" "SnapToTarget" true)
    (`self.K2_SetActorRelativeTransform` _returnvalue (`KismetMathLibrary.MakeTransform` (+ (* (0.0 10.0 0.0) _array_index) (0.0 0.0 1.0)) (struct :`Pitch` 90.0 :`Yaw` 90.0) (0.2 0.2 0.2)) false false)))

(fn `UserConstructionScript`)