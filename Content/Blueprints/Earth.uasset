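; Earth actor that slowly spins its cloud spheres and lights the globe according to the system date and time.
; Each tick, seconds since midnight set the sun yaw, while day of year sets pitch through a linear axial-tilt approximation starting at -23.44 degrees.
; The first two directional lights found in the level take this rotation, the second using the negated rotator.
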(event `self.ReceiveBeginPlay`
  (bind _outactors (`GameplayStatics.GetAllActorsOfClass` "/Script/Engine.DirectionalLight"))
  (set `self.DirLigRef` (`|GetArrayItem` _outactors))
  (set `self.DirLigRef2` (`|GetArrayItem` _outactors 1)))

(event `self.ReceiveTick`
  (params (DeltaSeconds :type "Float (single-precision)"))
  (`SceneComponent.K2_AddLocalRotation` (`self.Cloud_Spheres`) (struct :`Yaw` 0.001) false false)
  (bind _seconds (`self.GetTimeInSeconds`))
  (bind _newrot (`self.GetTimeRotation` _seconds))
  (`SceneComponent.K2_SetWorldRotation` (`Light.LightComponent` (`self.DirLigRef`)) _newrot false false)
  (`SceneComponent.K2_SetWorldRotation` (`Light.LightComponent` (`self.DirLigRef2`)) (`KismetMathLibrary.NegateRotator` _newrot) false false))

(fn `AxisCorrection`
  (returns (YRot :type "Float (double-precision)"))
  (bind _returndays (`self.GetDayOfYear`))
  (return (- (* _returndays 0.1284383561643836) 23.44)))

(fn `GetDayOfYear`
  (returns (ReturnDays :type Integer))
  (locals (Retur :type Integer))
  (bind (_year _month _day) (`KismetMathLibrary.BreakDateTime` (`KismetMathLibrary.Now`)))
  (for _index (range (+ _month 1))
    (set `local.Retur` (+ (`local.Retur`) (`|GetArrayItem` (`self.dagArray`) _index))))
  (bind _output_get (set `local.Retur` (+ _day (`local.Retur`))))
  (return _output_get))

(fn `GetTimeInSeconds`
  (returns (seconds :type Integer))
  (bind (_year _month _day _hour _minute _second) (`KismetMathLibrary.BreakDateTime` (`KismetMathLibrary.Now`)))
  (return (+ (* _hour 3600) (* _minute 60) _second)))

(fn `GetTimeRotation`
  (params (Sekunder :type Integer))
  (returns (NewRot :type "Rotator Structure"))
  (bind _yrot (`self.AxisCorrection`))
  (return (`KismetMathLibrary.MakeRotator` 0.0 _yrot (* Sekunder 0.004166666667))))

(fn `UserConstructionScript`)