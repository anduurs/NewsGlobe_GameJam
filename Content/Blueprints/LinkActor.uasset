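; LinkActor is a clickable 3D text link that shows its Title and opens its Link URL when clicked while hovered.
; On BeginPlay it creates a dynamic material for the text and binds to the GameController's interact dispatcher.
; HoverBegin and HoverEnd toggle the hover flag and the OverBloom material parameter, making the text glow.
; A click from the dispatcher launches the URL only while hovered.
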(event `self.ReceiveBeginPlay`
  (bind _textrender (`self.TextRender`))
  (`TextRenderComponent.K2_SetText` (`self.TextRender`) (`KismetTextLibrary.Conv_StringToText` (`self.Title`)))
  (bind _returnvalue (`PrimitiveComponent.CreateDynamicMaterialInstance` _textrender 0 (`PrimitiveComponent.GetMaterial` _textrender 0)))
  (set `self.Text Material Instance` _returnvalue)
  (bind _asgame_controller (cast `/Game/Blueprints/GameController` (`GameplayStatics.GetPlayerController` 0)))
  (add `/Game/Blueprints/GameController.InteractDispatcher` _asgame_controller (delegate `OnInteract`)))

(event `OnInteract`
  (params (Clicked :type Boolean))
  (if (and Clicked (`self.Hoover`))
    (`self.Click`)))

(event `self.Hover Begin`
  (`MaterialInstanceDynamic.SetScalarParameterValue` (`self.Text Material Instance`) "OverBloom" 50.0)
  (set `self.Hoover` true))

(event `self.Hover End`
  (`MaterialInstanceDynamic.SetScalarParameterValue` (`self.Text Material Instance`) "OverBloom" 1.0)
  (set `self.Hoover` false))

(event `self.Click`
  (`KismetSystemLibrary.LaunchURL` (`self.Link`)))

(fn `UserConstructionScript`)