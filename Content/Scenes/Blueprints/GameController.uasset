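; GameController is a drag-to-look controller that rotates the first player's pawn while the left mouse button is held.
; Press and release events toggle a flag, and the press also prints a debug message.
; While the flag is set, Tick adds input axis values to the pawn's pitch and yaw, clamping pitch to keep the view from flipping over.
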(event `self.ReceiveTick`
  (params (DeltaSeconds :type "Float (single-precision)"))
  (bind _returnvalue (`GameplayStatics.GetPlayerPawn` 0))
  (bind (_returnvalue_roll _returnvalue_pitch _returnvalue_yaw) (`KismetMathLibrary.BreakRotator` (`self.K2_GetActorRotation` _returnvalue)))
  (if (`self.Left Mouse Button Down`)
    (`self.K2_SetActorRotation` _returnvalue (`KismetMathLibrary.MakeRotator` 0.0 (`KismetMathLibrary.FClamp` (+ _returnvalue_pitch (`self.GetInputAxisKeyValue`)) -70.0 70.0) (+ _returnvalue_yaw (`self.GetInputAxisKeyValue`))) false)))

(event `Key|LeftMouseButton`
  (params (Key :type "Key Structure"))
  (:`Pressed`
    (set `self.Left Mouse Button Down` true)
    (`KismetSystemLibrary.PrintString` "Hello"))
  (:`Released`
    (set `self.Left Mouse Button Down` false)))

(event `Key|RightMouseButton`
  (params (Key :type "Key Structure")))

(fn `UserConstructionScript`)